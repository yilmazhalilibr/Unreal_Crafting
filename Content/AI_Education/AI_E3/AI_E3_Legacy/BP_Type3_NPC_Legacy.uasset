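; Legacy Type 3 AI NPC character that carries a weapon and adapts its movement to its combat state.
; On BeginPlay it spawns and attaches a weapon at WeaponSocket; damage from its HealthComponent plays a hit-react montage.
; State changes are forwarded to FirstPerson_AnimBP, while ModifyMovementSpeed tunes walk speed, acceleration and braking per state.
; Getters expose patrol route, death status and a fixed team ID; ModifyAimingStance is an empty stub.
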(event OnDamageTaken(HealthComponent)
  (Animation|PlayAnimMontage "/Game/AI_Education/AI_E3/Characters/Animations/Hit_React_1_Montage.Hit_React_1_Montage" 1.0 "None"))

(event Custom|NotifyStateChanged
  (params (New%20State :type ECombatState%20Enum :default "NewEnumerator0"))
  (bind (_anim_bp _success_) (CallFunction|GetAnimBlueprint))
  (if _success_
    (Class|AIHelperBPILegacy|NotifyStateChanged(Message) _anim_bp New%20State)))

(event EventBeginPlay
  (bind _self self)
  (Game|SpawnActorfromClass (Variables|Default|GetWeaponClass) (CallFunction|IdentityTransform) "AlwaysSpawn" _self _self)
  (Transformation|AttachComponentToComponent (Variables|Character|GetMesh) "WeaponSocket" "SnapToTarget" "SnapToTarget" "SnapToTarget" true))

(fn ConstructionScript)

(fn GetAnimBlueprint
  (bind _asfirst_person_anim_bp (Utilities|Casting|CastToFirstPerson_AnimBP (Components|SkeletalMesh|GetAnimInstance (Variables|Character|GetMesh)))
    (:then
      (return 0 true _asfirst_person_anim_bp))
    (:CastFailed
      (return 0 false 0))))

(fn ModifyMovementSpeed
  (params (Combat%20State :type ECombatState%20Enum :default "NewEnumerator0"))
  (Utilities|FlowControl|Sequence
    (:then_0
      (Variables|/Script/Engine.CharacterMovementComponent|SetMaxWalkSpeed (Variables|Character|GetCharacterMovement) (Utilities|Select :Index Combat%20State :NewEnumerator0 165.0 :NewEnumerator1 3e+02 :NewEnumerator2 4e+02 :NewEnumerator3 5.5e+02)))
    (:then_1
      (Variables|/Script/Engine.CharacterMovementComponent|SetMaxAcceleration (Variables|Character|GetCharacterMovement) (Utilities|Select :Index Combat%20State :NewEnumerator0 8e+02 :NewEnumerator1 8e+02 :NewEnumerator2 1e+03 :NewEnumerator3 1e+03)))
    (:then_2
      (Variables|/Script/Engine.CharacterMovementComponent|SetBrakingDecelerationWalking (Variables|Character|GetCharacterMovement) (Utilities|Select :Index Combat%20State :NewEnumerator0 7e+02 :NewEnumerator1 7e+02 :NewEnumerator2 8e+02 :NewEnumerator3 8e+02)))))

(fn ModifyAimingStance
  (params (IsAiming :type Boolean))
  (return))

(fn GetPatrolRoute
  (return (Variables|Default|GetMyPatrol)))

(fn GetIsDead
  (return (Default|IsDead (Variables|Default|GetHealthComponent))))

(fn GetTeamID
  (return 0))