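; Patrol route Blueprint that supplies NPCs with waypoints from the points of its PatrolPath spline.
; GetNextPointAsWorldPosition returns the world location of the spline point at the current PatrolIndex.
; IncrementPatrolPath advances that index with a modulo on the point count, so the route wraps back to the first point.
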(event Custom|IncrementPatrolPath
  (bind _result (Math|Integer|IncrementInt (Variables|Default|GetPatrolIndex))
    (:%20%20
      (Variables|Default|SetPatrolIndex (Math|Integer|%(Integer) _result (Spline|GetNumberOfSplinePoints (Variables|Default|GetPatrolPath)))))))

(fn ConstructionScript)

(fn GetNextPointasWorldPosition
  (return (Spline|GetLocationatSplinePoint (Variables|Default|GetPatrolPath) (Variables|Default|GetPatrolIndex) "World")))