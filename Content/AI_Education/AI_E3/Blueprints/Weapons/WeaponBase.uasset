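; Base weapon for the AI education project that fires from its muzzle when a fire request arrives.
; Each shot spawns a bullet actor and plays a fire sound, then runs a debug-drawn forward line trace on the Visibility channel out to weapon range.
; A trace hit applies point damage credited to the owner's instigator controller and reports a damage event for AI perception.
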(event Custom|OnFireRequested
  (bind _returnvalue (Components|GetOwner))
  (bind _muzzleposition (Variables|Default|GetMuzzlePosition))
  (bind _weapondamage (Variables|Default|GetWeaponDamage))
  (bind _returnvalue_2 (Game|GetInstigatorController _returnvalue))
  (bind _returnvalue_3 (Transformation|GetWorldLocation _muzzleposition))
  (CallFunction|FireRound)
  (Audio|PlaySoundatLocation "/Game/FirstPerson/Audio/FirstPersonTemplateWeaponFire02.FirstPersonTemplateWeaponFire02" _returnvalue_3 "0, 0, 0" 1.0 1.0 0.0 0 0 0)
  (bind (_outhit _returnvalue_4) (Collision|LineTraceByChannel _returnvalue_3 (+ _returnvalue_3 (* (Math|Vector|GetForwardVector _muzzleposition) (Variables|Default|GetWeaponRange))) "TraceTypeQuery1" false 0 "ForDuration"))
  (if _returnvalue_4
    (Game|Damage|ApplyPointDamage (.HitActor (Collision|BreakHitResult _outhit)) _weapondamage (.ImpactNormal (Collision|BreakHitResult _outhit)) _outhit _returnvalue_2 self "/Script/Engine.DamageType")
    (Class|AISenseDamage|ReportDamageEvent (.HitActor (Collision|BreakHitResult _outhit)) _returnvalue_2 _weapondamage (.Location (Collision|BreakHitResult _outhit)) "0, 0, 0" "None")))

(event Custom|FireRound
  (Game|SpawnActorfromClass (Variables|Default|GetBulletClass) (Transformation|GetWorldTransform (Variables|Default|GetMuzzlePosition)) "Undefined" 0 0))

(event EventBeginPlay)

(event Collision|EventActorBeginOverlap
  (params (OtherActor :type Actor%20Object%20Reference)))

(event EventTick
  (params (DeltaSeconds :type Float%20%28single-precision%29)))

(fn ConstructionScript)