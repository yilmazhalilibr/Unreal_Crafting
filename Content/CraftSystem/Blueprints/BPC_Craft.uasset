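; BPC_Craft is a crafting component that reads item recipes from ItemsDataTable.
; On BeginPlay it caches all row names into a unique list, then looks up the StoneIngot recipe without using the result.
; The lookup finds the name in the cached list, reads that row and returns its CraftMaterials map as separate material name and amount arrays, printing an error if the row is missing.
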(event EventBeginPlay
  ;[1 1 1] Initialize Function -Halil
  (CallFunction|GetDataTableRowNames)
  (CallFunction|GetRecipefromDataTable "StoneIngot"))

(fn GetDataTableRowNames
  (bind _outrownames (DataTable|GetDataTableRowNames "/Game/CraftSystem/DataTables/ItemsDataTable.ItemsDataTable"))
  (for _array_element _outrownames
    (Utilities|Array|AddUnique (Variables|Default|GetRowNamesList) _array_element))
  (return))

(fn GetRecipefromDataTable
  (params (RowName :type Name))
  (bind _returnvalue (Utilities|GetDataTableRow "/Game/CraftSystem/DataTables/ItemsDataTable.ItemsDataTable" (Utilities|Array|Get(acopy) (Variables|Default|GetRowNamesList) (Utilities|Array|FindItem (Variables|Default|GetRowNamesList) RowName)))
    (:then
      (bind _keys (Utilities|Map|Keys (.materials (.CraftMaterials (Utilities|Struct|BreakS_Recipes _returnvalue)))))
      (bind _values (Utilities|Map|Values (.materials (.CraftMaterials (Utilities|Struct|BreakS_Recipes _returnvalue)))))
      (return _keys _values))
    (:RowNotFound
      (Development|PrintString "Row isn't found the data table. Please check your data table or this code way."))))