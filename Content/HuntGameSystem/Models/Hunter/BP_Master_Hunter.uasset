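; Base hunter AI character for the hunt game, which spots hunts, rolls to attack them and plays rifle-fire and look-around montages.
; AI perception writes sighted hunts or lost-sight locations to the blackboard and notifies the hunt.
; HunterTriggered rolls hunt rate against a rating from league and gender-adjusted stats, adding league-based walk speed on each call.
; A successful roll sets AI_HunterController to attacking; the looping distance-check timer is unwired.
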(event OnPerceptionUpdated(AIPerception)
  (params (UpdatedActors :type Array%20of%20Actor%20Object%20References)))

(event OnTargetPerceptionUpdated(AIPerception)
  (params (Actor :type Actor%20Object%20Reference) (Stimulus :type AI%20Stimulus%20Structure))
  (CallFunction|HandleSightSense Actor Stimulus)
  (bind _asbp_master_hunt (Utilities|Casting|CastToBP_Master_Hunt Actor))
  (Default|OnHuntinSight _asbp_master_hunt self))

(event Custom|Attack
  (CallFunction|GetHuntDistance)
  (Animation|Montage|PlayMontage (Variables|Character|GetMesh) (Variables|Default|GetAnimFireMontage)
    (:OnCompleted
      _)
    (:OnInterrupted
      _))
  (Default|CallHunteronAttackEnd)
  (Development|PrintString "attack" true true "(R=0.000000,G=0.660000,B=1.000000,A=1.000000)" 0.5))

(event Custom|CheckInDistanceToHunt
  (bind _outactors (Actor|GetAllActorsOfClass "/Game/HuntGameSystem/Models/Hunt/BP_Master_Hunt.BP_Master_Hunt_C"))
  (if (<= (Math|Vector|Distance(Vector) (Transformation|GetWorldLocation (Variables|/Script/Engine.Character|GetMesh (Utilities|Array|Get(acopy) _outactors))) (Transformation|GetWorldLocation (Variables|Character|GetMesh))) 5e+02)
    (Variables|Default|SetHuntInDistance? true)
    (else
      (Variables|Default|SetHuntInDistance? false))))

(event Custom|CheckToAround
  (Animation|Montage|PlayMontage (Variables|Character|GetMesh) (Variables|Default|GetAnimCheckAroundMontage) 2.5))

(event EventBeginPlay
  (Variables|Default|SetAnimFireMontage "/Game/ExtraPackages/AnimStarterPack/AnimMontage_Fire_Rifle_Ironsights.AnimMontage_Fire_Rifle_Ironsights")
  (Variables|Default|SetAnimCheckAroundMontage "/Game/ExtraPackages/AnimStarterPack/CheckAroundMontage.CheckAroundMontage")
  (Pawn|SpawnDefaultController))

(fn ConstructionScript)

(fn CheckDistancetoHunt
  (params (Hunt :type Actor%20Object%20Reference))
  (if (<= (Transformation|GetDistanceTo Hunt) 4e+02)
    (bind _output_get (Variables|Default|SetHuntInDistance? true))
    (return _output_get)
    (else
      (bind _output_get_2 (Variables|Default|SetHuntInDistance? false))
      (return _output_get_2))))

(fn GetHuntDistance
  (bind _allhunts (Variables|Default|GetAllHunts))
  (bind _indistance_ (CallFunction|CheckDistancetoHunt (Utilities|Array|Get(acopy) _allhunts (Variables|Default|GetHuntIndex))))
  (if (< (Utilities|Array|Length _allhunts) (Variables|Default|GetHuntIndex))
    (Variables|Default|SetHuntIndex 0)
    (else
      (Math|Integer|IncrementInt (Variables|Default|GetHuntIndex)
        (:%20%20
          _))))
  (return _indistance_))

(fn CalculateDamageVisible
  (params (InGender :type Name) (InDamage :type Float%20%28single-precision%29) (InVisibleBonus :type Float%20%28single-precision%29))
  (LocalVariables|SetlocalDamage (Math|Float|Truncate InDamage))
  (LocalVariables|SetlocalVisibleBonus (Math|Float|Truncate InVisibleBonus))
  (switch name InGender
    (:man
      (return (+ (* (LocalVariables|GetlocalDamage) 0.5) (Math|Conversions|ToFloat(Integer) (LocalVariables|GetlocalDamage))) (+ (Math|Conversions|ToFloat(Integer) (LocalVariables|GetlocalVisibleBonus)) (* (LocalVariables|GetlocalVisibleBonus) 0.25))))
    (:woman
      (return (+ (* (LocalVariables|GetlocalDamage) 0.25) (Math|Conversions|ToFloat(Integer) (LocalVariables|GetlocalDamage))) (+ (Math|Conversions|ToFloat(Integer) (LocalVariables|GetlocalVisibleBonus)) (* (LocalVariables|GetlocalVisibleBonus) 0.5))))))

(fn CalculateWalkSpeed
  (params (localLeague :type Integer))
  (bind _charactermovement (Variables|Character|GetCharacterMovement))
  (Variables|/Script/Engine.CharacterMovementComponent|SetMaxWalkSpeed _charactermovement (Math|Conversions|ToFloat(Integer) (+ (* localLeague 50) (Math|Float|Truncate (Variables|/Script/Engine.CharacterMovementComponent|GetMaxWalkSpeed _charactermovement)))))
  (return))

(fn CalculateSightMatchRates
  (params (HuntRate :type Float%20%28single-precision%29) (HunterRate :type Float%20%28single-precision%29))
  (while (LocalVariables|GetlocalProcess?)
    (if (<= (Math|Conversions|ToFloat(Integer) (Math|Random|RandomIntegerinRange 10 100)) HuntRate)
      (LocalVariables|SetlocalHunt? true)
      (if (<= (Math|Conversions|ToFloat(Integer) (Math|Random|RandomIntegerinRange 0 100)) HunterRate)
        (LocalVariables|SetlocalHunter? true)
        (LocalVariables|SetlocalProcess? false)
        (return true)
        (else
          (LocalVariables|SetlocalProcess? false)
          (return false))))))

(fn CalculateRate
  (params (League :type Integer) (Damage :type Integer) (VisibleBonus :type Float%20%28single-precision%29))
  (bind _output_get (LocalVariables|SetlocalLeague League))
  (bind _output_get_2 (LocalVariables|SetlocalDamage Damage))
  (bind _output_get_3 (LocalVariables|SetlocalVisibleBonus VisibleBonus))
  (return (+ (* _output_get_3 0.35) (* _output_get_2 0.25) (* _output_get 5.0))))

(fn AttacktheCurrentHunt
  (bind _asai_hunter_controller (Utilities|Casting|CastToAI_HunterController (AI|GetAIController self)))
  (Default|SetStateasAttacking _asai_hunter_controller)
  (CallFunction|Attack))

(fn HunterTriggered
  (params (HuntRate :type Float%20%28single-precision%29))
  (bind _hunterrate (CallFunction|CalculateHunterProperties (Variables|Default|GetHunterProperties)))
  (bind _huntersaw_ (CallFunction|CalculateSightMatchRates HuntRate _hunterrate))
  (if _huntersaw_
    (CallFunction|ChecktoAround)
    (CallFunction|AttacktheCurrentHunt)
    (return true)
    (else
      (CallFunction|ChecktoAround)
      (return false))))

(fn GetAIControllerHunterState
  (params (State :type E_HunterAIStates%20Enum :default "NewEnumerator0"))
  (bind _asai_hunter_controller (Utilities|Casting|CastToAI_HunterController (AI|GetAIController self)))
  (switch Utilities|FlowControl|Switch|SwitchonE_HunterAIStates State
    (:NewEnumerator0
      (Default|SetStateasPassive _asai_hunter_controller))
    (:NewEnumerator1
      ;[1 1 1] Change later
      (bind _currenthunt (Default|CurrentHunt(FixLater) _asai_hunter_controller))
      (Default|SetStateasAttacking _asai_hunter_controller _currenthunt))))

(fn HunterStayinPlace
  (bind _charactermovement (Variables|Character|GetCharacterMovement))
  (Variables|Default|SetWalkSpeed (Variables|/Script/Engine.CharacterMovementComponent|GetMaxWalkSpeed _charactermovement))
  (Variables|/Script/Engine.CharacterMovementComponent|SetMaxWalkSpeed _charactermovement 0.0)
  (return))

(fn HunterContunieinWay
  (Variables|/Script/Engine.CharacterMovementComponent|SetMaxWalkSpeed (Variables|Character|GetCharacterMovement) (Variables|Default|GetWalkSpeed))
  (return))

(fn HandleSightSense
  (params (Actor :type Actor%20Object%20Reference) (Stimulus :type AI%20Stimulus%20Structure))
  (bind _returnvalue (Class|AIPerceptionSystem|GetSenseClassforStimulus Stimulus))
  (if (== _returnvalue "/Script/AIModule.AISense_Sight")
    (bind _outactors (Actor|GetAllActorsOfClass "/Game/HuntGameSystem/Models/HuntGame_Manager.HuntGame_Manager_C"))
    (bind (_array_element _array_index) (Utilities|Array|ForEachLoopwithBreak (Variables|/Game/HuntGameSystem/Models/HuntGame_Manager.HuntGame_Manager_C|GetHuntsList (Utilities|Array|Get(acopy) _outactors)) :!label _label)
      (:LoopBody
        (if (== Actor (Utilities|Array|Get(acopy) (Variables|/Game/HuntGameSystem/Models/HuntGame_Manager.HuntGame_Manager_C|GetHuntsList (Utilities|Array|Get(acopy) _outactors)) _array_index))
          (goto _label Break)))
      (:Completed
        (AI|Components|Blackboard|SetValueasObject (Variables|/Script/AIModule.AIController|GetBlackboard (AI|GetAIController self)) (Variables|Default|GetHuntKey) (select (.bsuccessfullysensed Stimulus) _array_element 0))
        (if (not (.bsuccessfullysensed Stimulus))
          (AI|Components|Blackboard|SetValueasVector (AI|GetBlackboard self) (Variables|Default|GetHuntVectorKey) (.stimuluslocation Stimulus)))))
    (else
      (return))))

(fn CalculateHunterProperties
  (params (Hunter%20Properties :type S%20Hunter%20Properties%20Structure))
  (bind (_league _rank _basedamage _visiblebonus _gender) (Utilities|Struct|BreakS_HunterProperties Hunter%20Properties))
  (LocalVariables|SetlocalLeague _league)
  (LocalVariables|SetlocalRank _rank)
  (bind _output_get (LocalVariables|SetlocalDamage _basedamage))
  (bind _output_get_2 (LocalVariables|SetlocalVisibleBonus (Math|Conversions|ToFloat(Integer) _visiblebonus)))
  (bind (_outdamage _outvisiblebonus) (CallFunction|CalculateDamageVisible _gender (Math|Conversions|ToFloat(Integer) _output_get) _output_get_2))
  (LocalVariables|SetlocalDamage (Math|Float|Truncate _outdamage))
  (LocalVariables|SetlocalVisibleBonus _outvisiblebonus)
  (CallFunction|CalculateWalkSpeed (LocalVariables|GetlocalLeague))
  (bind _hunterrate (CallFunction|CalculateRate (LocalVariables|GetlocalLeague) (LocalVariables|GetlocalDamage) (LocalVariables|GetlocalVisibleBonus)))
  (return _hunterrate))

(fn GetPatrolRoute
  (return (Variables|AI|GetPatrolRoute)))